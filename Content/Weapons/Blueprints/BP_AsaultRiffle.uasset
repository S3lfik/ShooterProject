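; Assault rifle weapon Blueprint that fires automatically while the trigger is held and ammo remains.
; PullTrigger drives a Gate and RetriggerableDelay loop that spawns a projectile, muzzle flash and sound at the MuzzleFlash socket, plays the fire animation and decrements ammo.
; WeaponInfo supplies clip size, projectile class and bullet speed.
; ToReload plays an animation and refills the clip after a fixed placeholder delay, not an animation-complete callback.
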(event `self.ReceiveBeginPlay`
  (bind (_weaponinfo_projectileclass _weaponinfo_clipsize) (break `/Game/Weapons/Blueprints/struct_WeaponInfo` (`self.WeaponInfo`)))
  (`parent.ReceiveBeginPlay`)
  (set `self.AmmoCount` _weaponinfo_clipsize))

(event `self.PullTrigger`
  (`|ExecutionSequence`
    (:`then_0`
      (goto _label_2 :!via `Open`))
    (:`then_1`
      (if (> (`self.AmmoCount`) 0) :!label _label
        (`/Engine/EditorBlueprintResources/StandardMacros.Gate` true :!label _label_2
          (:`Exit`
            (`self.CreateBullet`)
            (`self.CreateFX`)
            (`self.CreateFireSound`)
            (`SkeletalMeshComponent.PlayAnimation` (`self.Weapon`) "/Game/Weapons/Anims/Fire_Rifle_W.Fire_Rifle_W" false)
            (bind _result (`/Engine/EditorBlueprintResources/StandardMacros.DecrementInt` (`self.AmmoCount`))
              (:`  `
                (bind _output_get (set `self.AmmoCount` _result))
                (`KismetSystemLibrary.PrintString` (`KismetStringLibrary.Conv_IntToString` _output_get))
                (`KismetSystemLibrary.RetriggerableDelay` (`self.FireDelay`))
                (goto _label)))))
        (else
          (goto _label_2 :!via `Close`))))))

(event `self.ReleaseTrigger`
  (goto _label_2 :!via `Close`))

(event `self.ToReload`
  (bind (_weaponinfo_projectileclass _weaponinfo_clipsize) (break `/Game/Weapons/Blueprints/struct_WeaponInfo` (`self.WeaponInfo`)))
  (`SkeletalMeshComponent.PlayAnimation` (`self.Weapon`) "/Game/Weapons/Anims/Reload_Rifle_Ironsights_W.Reload_Rifle_Ironsights_W" false)
  ;[1 1 1] To remake into callback for animation complete
  (`KismetSystemLibrary.Delay` 0.2)
  (set `self.AmmoCount` _weaponinfo_clipsize))

(event `self.onApplyReload`)

(fn `CreateBullet`
  (bind (_weaponinfo_projectileclass _weaponinfo_clipsize _weaponinfo_firerate _weaponinfo_recoil _weaponinfo_bulletspeed) (break `/Game/Weapons/Blueprints/struct_WeaponInfo` (`self.WeaponInfo`)))
  (bind _returnvalue (`|SpawnActorFromClass` _weaponinfo_projectileclass (`SceneComponent.GetSocketTransform` (`self.Weapon`) "MuzzleFlash" "RTS_World") "AlwaysSpawn" "OverrideRootScale" null null))
  (`/Engine/EditorBlueprintResources/StandardMacros.IsValid` _returnvalue
    (:`Is Valid`
      (`/Game/Weapons/Blueprints/Projectiles/BP_ProjectileBase.SetBulletSpeed` _returnvalue _weaponinfo_bulletspeed))))

(fn `CreateFireSound`
  (`GameplayStatics.PlaySoundAtLocation` "/Game/Weapons/Sound/Rifle/RifleB_Fire01.RifleB_Fire01" (`SceneComponent.GetSocketLocation` (`self.Weapon`) "MuzzleFlash") (struct) 1.0 1.0 0.0 null null null))

(fn `CreateFX`
  (bind (_returnvalue_location _returnvalue_rotation _returnvalue_scale) (`KismetMathLibrary.BreakTransform` (`SceneComponent.GetSocketTransform` (`self.Weapon`) "MuzzleFlash" "RTS_World")))
  (`GameplayStatics.SpawnEmitterAtLocation` "/Game/Weapons/FX/P_AssaultRifle_MuzzleFlash.P_AssaultRifle_MuzzleFlash" _returnvalue_location _returnvalue_rotation _returnvalue_scale))

(fn `UserConstructionScript`
  (`parent.UserConstructionScript`))