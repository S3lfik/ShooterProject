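; Assault rifle projectile that shows a tracer and damages what it hits.
; BeginPlay attaches the tracer emitter to the projectile mesh.
; Hit applies fixed point damage with player 0's controller as instigator, spawns a pooled impact effect along the surface normal, removes any valid TrailFX and destroys itself.
; Actor and mesh overlaps only print the other actor's name for debugging.
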(event `self.ReceiveBeginPlay`
  (bind (_returnvalue_location _returnvalue_rotation _returnvalue_scale) (`KismetMathLibrary.BreakTransform` (`self.GetTransform`)))
  (`parent.ReceiveBeginPlay`)
  (`GameplayStatics.SpawnEmitterAttached` "/Game/Weapons/FX/P_AssaultRifle_Tracer.P_AssaultRifle_Tracer" (`self.ProjectileMesh`) "None" _returnvalue_location _returnvalue_rotation _returnvalue_scale "KeepWorldPosition"))

(event `self.ReceiveActorBeginOverlap`
  (params (OtherActor :type "Actor Object Reference"))
  (`KismetSystemLibrary.PrintString` (`KismetSystemLibrary.GetObjectName` OtherActor)))

(event `self.ProjectileMesh.OnComponentBeginOverlap`
  (params (OverlappedComponent :type "PrimitiveComponent Object Reference") (OtherActor :type "Actor Object Reference") (OtherComp :type "PrimitiveComponent Object Reference") (OtherBodyIndex :type Integer) (bFromSweep :type Boolean) (SweepResult :type "HitResult Structure (by ref)"))
  (`KismetSystemLibrary.PrintString` (`KismetSystemLibrary.GetObjectName` OtherActor)))

(event `self.ReceiveHit`
  (params (MyComp :type "PrimitiveComponent Object Reference") (Other :type "Actor Object Reference") (OtherComp :type "PrimitiveComponent Object Reference") (bSelfMoved :type Boolean) (HitLocation :type "Vector Structure") (HitNormal :type "Vector Structure") (NormalImpulse :type "Vector Structure") (Hit :type "HitResult Structure (by ref)"))
  (bind _trailfx (`self.TrailFX`))
  (`GameplayStatics.ApplyPointDamage` Other 100.0 (`self.K2_GetActorLocation`) Hit (`GameplayStatics.GetPlayerController` 0) (`self.GetOwner`) "/Game/Weapons/Blueprints/Projectiles/BP_BaseDamageType.BP_BaseDamageType_C")
  (`GameplayStatics.SpawnEmitterAtLocation` "/Game/Weapons/FX/P_Impact_01.P_Impact_01" HitLocation (`KismetMathLibrary.Quat_Rotator` (`KismetMathLibrary.Conv_VectorToQuaterion` HitNormal)) (1.0 1.0 1.0) true "AutoRelease")
  (`/Engine/EditorBlueprintResources/StandardMacros.IsValid` _trailfx
    (:`Is Valid`
      (`ActorComponent.K2_DestroyComponent` _trailfx))
    (:`Is Not Valid`
      _))
  (`self.K2_DestroyActor`))

(fn `UserConstructionScript`
  (`parent.UserConstructionScript`))