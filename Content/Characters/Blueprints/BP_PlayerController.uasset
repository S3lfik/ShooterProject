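; Player controller that creates a crosshair widget and makes the possessed MasterPoseCharacter aim at whatever lies under it.
; On possess it caches the character and its AimingComponent, clearing both on unpossess.
; Each tick it deprojects the crosshair's screen position and line traces on the Camera channel from the character's current camera, with debug drawing enabled.
; On a hit, the impact point goes to the AimingComponent's AimAt.
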(event `self.ReceiveBeginPlay`
  (`|ExecutionSequence`
    (:`then_0`
      (bind _returnvalue (`|CreateWidget` "/Game/UI/UMG_Crosshair.UMG_Crosshair_C" self))
      (bind _output_get (set `self.Crosshair` _returnvalue))
      (`UserWidget.AddToViewport` _output_get 0))))

(event `self.ReceivePossess`
  (params (PossessedPawn :type "Pawn Object Reference"))
  (bind _asmaster_pose_character (cast `/Game/Characters/Blueprints/MasterPoseCharacter` PossessedPawn))
  (set `self.PossessedCharacter` _asmaster_pose_character)
  (set `self.AimingComp` (`/Game/Characters/Blueprints/MasterPoseCharacter.AimingComponent` _asmaster_pose_character)))

(event `self.ReceiveUnPossess`
  (params (UnpossessedPawn :type "Pawn Object Reference"))
  (set `self.PossessedCharacter` null)
  (set `self.AimingComp` null))

(event `self.ReceiveTick`
  (params (DeltaSeconds :type "Float (single-precision)"))
  (`self.AimTowardsCrosshair`))

(fn `AimTowardsCrosshair`
  (bind _aimingcomp (`self.AimingComp`)
    (:`then`
      (bind (_lookatpoint _hitsanything) (`self.GetLookAtPointHitResult`))
      (if _hitsanything
        (`/Game/Characters/Blueprints/BP_AimingComponent.AimAt` _aimingcomp (`.ImpactPoint` (`GameplayStatics.BreakHitResult` _lookatpoint)))))
    (:`else`
      (return))))

(fn `GetLookAtPointHitResult`
  (returns (LookAtPoint :type "HitResult Structure") (HitsAnything :type Boolean))
  (bind _returnvalue (`self.K2_GetPawn`))
  (bind _returnvalue_2 (`GameplayStatics.MakeHitResult` false))
  (bind (_worldposition _worlddirection _returnvalue_3) (`GameplayStatics.DeprojectScreenToWorld` self (`/Game/UI/UMG_Crosshair.GetCrosshairLocation` (`self.Crosshair`))))
  (if _returnvalue_3
    (bind _asmaster_pose_character (cast `/Game/Characters/Blueprints/MasterPoseCharacter` _returnvalue)
      (:`then`
        (bind (_outhit _returnvalue_4) (`KismetSystemLibrary.LineTraceSingle` (`SceneComponent.K2_GetComponentLocation` (`/Game/Characters/Blueprints/MasterPoseCharacter.CurrentCamera` _asmaster_pose_character)) (+ _worldposition (* _worlddirection 10000.0)) "TraceTypeQuery2" false (`|MakeArray` _returnvalue :!type "Actor Object Reference") "ForDuration" true (struct :`R` 1.0 :`A` 1.0) (struct :`G` 1.0 :`A` 1.0) 0.1))
        (return _outhit _returnvalue_4))
      (:`CastFailed`
        (return _returnvalue_2 false)))
    (else
      (return _returnvalue_2 false))))

(fn `UserConstructionScript`)