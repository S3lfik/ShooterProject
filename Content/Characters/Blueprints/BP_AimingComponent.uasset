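; Character aiming component that relays fire, cease-fire and reload commands to its Weapon, printing debug text for trigger pulls and releases.
; AimAt rotates the weapon from its MuzzleFlash socket toward a supplied location in two of the aiming states, drawing a debug line.
; BeginPlay caches the player controller, used only by an unconnected older version of the aim logic that reads the controller's look-at hit result.
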(event `self.ReceiveBeginPlay`
  (bind _asbp_player_controller (cast `/Game/Characters/Blueprints/BP_PlayerController` (`GameplayStatics.GetPlayerController` 0)))
  (set `self.CurrentPlayerController` _asbp_player_controller))

(event `self.ReceiveTick`
  (params (DeltaSeconds :type "Float (single-precision)")))

(event `Fire`
  (bind _weapon (`self.Weapon`))
  (`/Engine/EditorBlueprintResources/StandardMacros.IsValid` _weapon
    (:`Is Valid`
      (`/Game/Weapons/Blueprints/BP_WeaponBase.PullTrigger` _weapon)
      (`KismetSystemLibrary.PrintString` "Pull Trigger"))))

(event `CeaseFire`
  (bind _weapon (`self.Weapon`))
  (`/Engine/EditorBlueprintResources/StandardMacros.IsValid` _weapon
    (:`Is Valid`
      (`/Game/Weapons/Blueprints/BP_WeaponBase.ReleaseTrigger` _weapon)
      (`KismetSystemLibrary.PrintString` "Release Trigger"))))

(event `Reload`
  (bind _weapon (`self.Weapon`))
  (`/Engine/EditorBlueprintResources/StandardMacros.IsValid` _weapon
    (:`Is Valid`
      (`/Game/Weapons/Blueprints/BP_WeaponBase.ToReload` _weapon))))

(fn `AimAt`
  (params (AimingLocation :type "Vector Structure"))
  (bind _weapon (`self.Weapon`))
  (bind _returnvalue (`SceneComponent.GetSocketLocation` (`/Game/Weapons/Blueprints/BP_WeaponBase.Weapon` _weapon) "MuzzleFlash"))
  (if (or (`|EnumEquality` (`self.EAimingState`) "NewEnumerator1") (`|EnumEquality` (`self.EAimingState`) "NewEnumerator2"))
    (if true
      (`KismetSystemLibrary.DrawDebugLine` _returnvalue AimingLocation (struct :`R` 0.123761 :`G` 0.737067 :`B` 1.0 :`A` 1.0) 0.1 1.0)
      (`Actor.K2_SetActorRotation` _weapon (`KismetMathLibrary.FindLookAtRotation` _returnvalue AimingLocation) false))))