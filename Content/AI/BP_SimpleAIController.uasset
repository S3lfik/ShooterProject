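; AI controller that runs the BH_SimpleAI behavior tree on its pawn, caches the first patrol path, and manages battle state.
; Perception sightings of MasterPoseCharacters write target, last-seen location and battle flag to the blackboard, without calling the team check.
; Losing sight starts a memory timer that clears that state on expiry.
; Tick yaws the pawn toward its target, marked as a placeholder for aim logic.
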(event `self.ReceiveBeginPlay`
  (bind _outactors (`GameplayStatics.GetAllActorsOfClass` "/Game/AI/BP_PatrolPath.BP_PatrolPath_C"))
  (set `self.PatrolPath` (`|GetArrayItem` _outactors)))

(event `self.ReceiveTick`
  (params (DeltaSeconds :type "Float (single-precision)"))
  (`|ExecutionSequence`
    (:`then_0`
      (if (`self.BTKeyIsInBattle`)
        (if (<= (`self.TargetInterestSpan`) 0.0)
          (set `self.BTKeyIsInBattle` false)
          (set `self.TargetActor` null)
          ;[1 1 1] Replace/adjust with AimAt logic later
          (`self.UpdateRotation` :!label _label))))
    (:`then_1`
      (goto _label))))

(event `self.ReceivePossess`
  (params (PossessedPawn :type "Pawn Object Reference"))
  (set `self.PossessedActor` PossessedPawn)
  (`self.RunBehaviorTree` "/Game/AI/BH_SimpleAI.BH_SimpleAI"))

(event `self.ReceiveUnPossess`
  (params (UnpossessedPawn :type "Pawn Object Reference"))
  (set `self.PossessedActor` null))

(event `self.AIPerception.OnTargetPerceptionUpdated`
  (params (Actor :type "Actor Object Reference") (Stimulus :type "AIStimulus Structure"))
  (bind (_age _expirationage _strength _stimuluslocation _receiverlocation _tag _bsuccessfullysensed) (break `AIStimulus` Stimulus))
  (`|ExecutionSequence`
    (:`then_0`
      (if _bsuccessfullysensed
        (bind _asmaster_pose_character (cast `/Game/Characters/Blueprints/MasterPoseCharacter` Actor))
        (`KismetSystemLibrary.K2_ClearAndInvalidateTimerHandle` (`self.TargetMemoryTimer`))
        (`self.EnterBattleMode` _asmaster_pose_character _stimuluslocation)
        (`KismetSystemLibrary.PrintString` "Target received")
        (else
          (bind _returnvalue (`KismetSystemLibrary.K2_SetTimerDelegate` (delegate `StartTimerCooldown`) (`self.TargetInterestSpan`)))
          (set `self.TargetMemoryTimer` _returnvalue)
          (`KismetSystemLibrary.PrintString` "Target Lost"))))
    (:`then_1`
      (if (<= _age 0.0)
        (set `self.BTKeyIsTargetVisible` false)))))

(event `StartTimerCooldown`
  (`self.QuitBattleState`))

(fn `EnterBattleMode`
  (params (TargetActor :type "Actor Object Reference") (TargetSeenLocation :type "Vector Structure"))
  (set `self.BTKeyTargetLastSeenLocation` TargetSeenLocation)
  (bind _output_get (set `self.TargetActor` TargetActor))
  (`BlackboardComponent.SetValueAsObject` (`AIBlueprintHelperLibrary.GetBlackboard` null) (`self.BTKeyNameTargetActor`) _output_get)
  (`BlackboardComponent.SetValueAsVector` (`self.Blackboard`) (`self.BTKeyNameTargetLastSeenLocation`) (`self.BTKeyTargetLastSeenLocation`))
  (set `self.BTKeyIsInBattle` true)
  (`BlackboardComponent.SetValueAsBool` (`self.Blackboard`) (`self.BTKeyNameIsInBattle`) (`self.BTKeyIsInBattle`))
  (return))

(fn `IsActorEnemy`
  (params (NewParam :type "Actor Object Reference"))
  (returns (IsEnemy :type Boolean))
  (bind _possessedactor (`self.PossessedActor`))
  (bind _asmaster_pose_character (cast `/Game/Characters/Blueprints/MasterPoseCharacter` NewParam)
    (:`then`
      (`/Engine/EditorBlueprintResources/StandardMacros.IsValid` _possessedactor
        (:`Is Valid`
          (bind _asbp_simple_ai (cast `/Game/AI/BP_SimpleAI` _possessedactor)
            (:`then`
              (return (not (`|EnumEquality` (`/Game/AI/BP_SimpleAI.Team` _asbp_simple_ai) (`/Game/Characters/Blueprints/MasterPoseCharacter.Team` _asmaster_pose_character)))))
            (:`CastFailed`
              _)))
        (:`Is Not Valid`
          _)))
    (:`CastFailed`
      _))
  (return false))

(fn `QuitBattleState`
  (bind _output_get (set `self.BTKeyIsInBattle` false))
  (`BlackboardComponent.SetValueAsBool` (`self.Blackboard`) (`self.BTKeyNameIsInBattle`) _output_get)
  (bind _output_get_2 (set `self.BTKeyTargetLastSeenLocation` (0.0 0.0 0.0)))
  (`BlackboardComponent.SetValueAsVector` (`self.Blackboard`) (`self.BTKeyNameTargetLastSeenLocation`) _output_get_2)
  (bind _output_get_3 (set `self.TargetActor` null))
  (`BlackboardComponent.SetValueAsObject` (`self.Blackboard`) (`self.BTKeyNameTargetActor`) _output_get_3)
  (return))

(fn `UpdateRotation`
  (bind _targetactor (`self.TargetActor`))
  (bind _possessedactor (`self.PossessedActor`))
  (`/Engine/EditorBlueprintResources/StandardMacros.IsValid` _targetactor
    (:`Is Valid`
      (`/Engine/EditorBlueprintResources/StandardMacros.IsValid` _possessedactor
        (:`Is Valid`
          (`self.K2_SetActorRotation` _possessedactor (`KismetMathLibrary.MakeRotator` 0.0 0.0 (.yaw (`KismetMathLibrary.FindLookAtRotation` (`self.K2_GetActorLocation` _possessedactor) (`self.K2_GetActorLocation` _targetactor)))) false)
          (return))
        (:`Is Not Valid`
          (return))))
    (:`Is Not Valid`
      (return))))

(fn `UserConstructionScript`)